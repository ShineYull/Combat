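; AC_Combat is a combat component for a Character owner that plays melee-style combo attacks on the ground and a single attack in the air.
; TriggerAttack picks the attack from the falling state, and flags block re-triggering.
; Ground attacks cycle through a montage array, with montage notify windows reopening input for chaining and completion resetting the combo.
; The Landed delegate resets both attacks and cuts short a playing air montage.
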(event `self.ReceiveBeginPlay`
  (bind _ascharacter (cast `Character` (`self.GetOwner`)))
  (set `self.CharacterMesh` (`Character.Mesh` _ascharacter))
  (set `self.CharacterActor` _ascharacter)
  (add `Character.LandedDelegate` (`self.CharacterActor`) (`|CreateDelegate` :!event `OnCharacterLanded`)))

(event `GroundAttack`
  (`self.bCanAttack`
    (:`then`
      (set `self.bCanAttack` false)
      (bind _notifyname (`|PlayMontage` (`self.CharacterMesh`) (`|GetArrayItem` (`self.AttackAnims`) (`self.AttackIndexCurrent`)))
        (:`then`
          (set `self.AttackIndexCurrent` (`KismetMathLibrary.SelectInt` (+ (`self.AttackIndexCurrent`) 1) 0 (< (`self.AttackIndexCurrent`) (`KismetArrayLibrary.Array_LastIndex` (`self.AttackAnims`))))))
        (:`OnCompleted`
          (set `self.bCanAttack` true)
          (set `self.AttackIndexCurrent` 0))
        (:`OnNotifyBegin`
          (switch `name` _notifyname
            (:`ComboInputWindow`
              (set `self.bCanAttack` true))))
        (:`OnNotifyEnd`
          (switch `name` _notifyname
            (:`ComboInputWindow`
              (set `self.bCanAttack` false))))))
    (:`else`)))

(event `AirAttack`
  (`self.bCanAirAttack`
    (:`then`
      (set `self.bCanAirAttack` false)
      (`|PlayMontage` (`self.CharacterMesh`) (`self.AirAttackAnim`)
        (:`OnBlendOut`
          (set `self.bCanAirAttack` true))))
    (:`else`)))

(event `TriggerAttack`
  (if (`NavMovementComponent.IsFalling` (`Character.CharacterMovement` (`self.CharacterActor`)))
    (`self.AirAttack`)
    (else
      (`self.GroundAttack`))))

(event `OnCharacterLanded`
  (params (Hit :type "HitResult Structure (by ref)"))
  (set `self.bCanAirAttack` true)
  (set `self.bCanAttack` true)
  (set `self.AttackIndexCurrent` 0)
  (if (== (`Character.GetCurrentMontage` (`self.CharacterActor`)) (`self.AirAttackAnim`))
    (`Character.StopAnimMontage` (`self.CharacterActor`) null)))