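; Actor component that gives its owning Character a hit stop, with slowed time, mesh shake and an optional flash.
; BeginHitStop sets custom time dilation, applies a dynamic overlay material and starts shake and duration timers.
; Shake steps offset the mesh along the camera's right axis in actor space, scaled by a curve over elapsed time.
; EndHitStop restores mesh location, time dilation and overlay.
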(event `self.ReceiveBeginPlay`
  (bind _ascharacter (cast `Character` (`self.GetOwner`)))
  (bind _output_get (set `self.CharacterActor` _ascharacter))
  (bind _output_get_2 (set `self.Mesh` (`Character.Mesh` _output_get)))
  (set `self.MeshDefaultRelativeLoc` (`SceneComponent.RelativeLocation` _output_get_2))
  (bind _returnvalue (`KismetMaterialLibrary.CreateDynamicMaterialInstance` "/Game/Combat/M_HitFlash.M_HitFlash"))
  (bind _output_get_3 (set `self.HitFlashMaterial` _returnvalue))
  (`MaterialInstanceDynamic.SetScalarParameterValue` _output_get_3 "Speed" 20.0))

(event `BeginHitStop`
  (params (InDuration :type "Float (double-precision)") (InTimeDilation :type "Float (double-precision)") (InShakeSpeed :type "Float (double-precision)") (InShakeAmplitude :type "Float (double-precision)") (InFlash :type Boolean))
  (set `self.Flash` InFlash)
  (set `self.ShakeAmplitude` InShakeAmplitude)
  (bind _returnvalue (`KismetSystemLibrary.K2_SetTimerDelegate` (`|CreateDelegate` :!event `ApplyMeshShakeStep`) (/ 1.0 InShakeSpeed) true))
  (set `self.ShakeTimer` _returnvalue)
  (set `Actor.CustomTimeDilation` InTimeDilation (`self.CharacterActor`))
  (bind _returnvalue_2 (`KismetSystemLibrary.K2_SetTimerDelegate` (`|CreateDelegate` :!event `EndHitStop`) InDuration))
  (set `self.HitStopTimer` _returnvalue_2)
  (set `self.HitStopDuration` InDuration)
  (`self.Flash`
    (:`then`
      (`MeshComponent.SetOverlayMaterial` (`self.Mesh`) (`self.HitFlashMaterial`)))
    (:`else`)))

(event `EndHitStop`
  (`KismetSystemLibrary.K2_ClearAndInvalidateTimerHandle` (`self.ShakeTimer`))
  (`SceneComponent.K2_SetRelativeLocation` (`self.Mesh`) (`self.MeshDefaultRelativeLoc`) false true)
  (set `Actor.CustomTimeDilation` 1.0 (`self.CharacterActor`))
  (`self.Flash`
    (:`then`
      (`MeshComponent.SetOverlayMaterial` (`self.Mesh`) null))
    (:`else`)))

(event `ApplyMeshShakeStep`
  (bind (_returnvalue_x _returnvalue_y) (`KismetMathLibrary.BreakVector` (`KismetMathLibrary.InverseTransformDirection` (`Actor.GetTransform` (`self.CharacterActor`)) (`Actor.GetActorRightVector` (`PlayerController.PlayerCameraManager` (`GameplayStatics.GetPlayerController` 0))))))
  (`SceneComponent.K2_SetRelativeLocation` (`self.Mesh`) (+ (`self.MeshDefaultRelativeLoc`) (* (`KismetMathLibrary.MakeVector` _returnvalue_x _returnvalue_y) (* (`self.ShakeAmplitude`) (`self.OffsetDirection`)) (`CurveFloat.GetFloatValue` (`self.ShakeResolve`) (/ (`KismetSystemLibrary.K2_GetTimerElapsedTimeHandle` (`self.HitStopTimer`)) (`self.HitStopDuration`))))) false true)
  (`/Engine/EditorBlueprintResources/StandardMacros.NegateFloat` (`self.OffsetDirection`)))